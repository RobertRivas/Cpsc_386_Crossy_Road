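; BP_Dirt_road_Spawner builds a run of dirt road by spawning BP_Dirt_road segments end to end.
; SpawnInitialDirtRoad loops to place the first segment at the world origin and each next one at the latest segment's DirtRoadSpawnPoint.
; Each segment receives a reference back to the spawner.
; BeginPlay is empty and the initial spawn call is disconnected, so nothing here starts spawning; leftover random-selection nodes are also unused.
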(event `self.ReceiveBeginPlay`)

(fn `Spawn_Dirt_Road`
  (params (spawn_location :type "Vector Structure"))
  (bind _returnvalue (`|SpawnActorFromClass` "/Game/blueprints/BP_Dirt_road.BP_Dirt_road_C" (`KismetMathLibrary.MakeTransform` spawn_location) "Undefined" "OverrideRootScale" null null))
  (bind _output_get (set `self.newdirtroad` _returnvalue))
  (set `/Game/blueprints/BP_Dirt_road.dirt_road_Spawner` self _output_get))

(fn `spawn_Dirt_road_at _spawn_point`
  (`self.Spawn_Dirt_Road` (`SceneComponent.K2_GetComponentLocation` (`/Game/blueprints/BP_Dirt_road.dirt_road_spawn_point` (`self.newdirtroad`)))))

(fn `Spawn_initial_Dirt_road`
  (for _ (range 4)
    (`/Engine/EditorBlueprintResources/StandardMacros.IsValid` (`self.newdirtroad`)
      (:`Is Valid`
        (`self.spawn_Dirt_road_at _spawn_point`))
      (:`Is Not Valid`
        (`self.Spawn_Dirt_Road` (0.0 0.0 0.0))))))

(fn `UserConstructionScript`)