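; BP_Grass_Spawner is a spawner that lays BP_Grass actors in a chain, though nothing in its own event graph currently triggers it.
; SpawnInitialGrass loops, placing grass at the world origin if none exists, otherwise at the last piece's SpawnPoint.
; SpawnGrass stores each new actor as Newgrass and gives it a back-reference to the spawner.
; Disconnected nodes hold leftover random-choice and road-spawning logic.
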(event `self.ReceiveBeginPlay`)

(fn `Spawn_Grass`
  (params (spawn_location :type "Vector Structure"))
  (bind _returnvalue (`|SpawnActorFromClass` "/Game/blueprints/BP_Grass.BP_Grass_C" (`KismetMathLibrary.MakeTransform` spawn_location) "Undefined" "OverrideRootScale" null null))
  (bind _output_get (set `self.newgrass` _returnvalue))
  (set `/Game/blueprints/BP_Grass.Grass_Spawner` self _output_get))

(fn `spawn_grass_at _spawn_point`
  (`self.Spawn_Grass` (`SceneComponent.K2_GetComponentLocation` (`/Game/blueprints/BP_Grass.spawn_point` (`self.newgrass`)))))

(fn `Spawn_initial_grass`
  (for _ (range 4)
    (`/Engine/EditorBlueprintResources/StandardMacros.IsValid` (`self.newgrass`)
      (:`Is Valid`
        (`self.spawn_grass_at _spawn_point`))
      (:`Is Not Valid`
        (`self.Spawn_Grass` (0.0 0.0 0.0))))))

(fn `UserConstructionScript`)