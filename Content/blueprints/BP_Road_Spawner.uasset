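; BP_Road_Spawner is an actor with functions for spawning floor pieces, nominally road or grass, though both spawn BP_Road and store it in Newroad.
; Chaining helpers place a piece at the SpawnPoint of Newroad or Newgrass, but Newgrass is never set here.
; SpawnInitialGrass loops this with an origin fallback, and FloorPartToSpawn randomly picks either type at the origin.
; Event graph and construction script are empty, so nothing here triggers spawning.
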(event `self.ReceiveBeginPlay`)

(fn `Floor_Part _To_Spawn`
  (switch `int` (`KismetMathLibrary.RandomIntegerInRange` 0 1)
    (:`0`
      (`self.Spawn_Road` (0.0 0.0 0.0)))
    (:`1`
      (`self.Spawn_Grass` (0.0 0.0 0.0)))))

(fn `Spawn_Grass`
  (params (spawn_location :type "Vector Structure"))
  (bind _returnvalue (`|SpawnActorFromClass` "/Game/blueprints/BP_Road.BP_Road_C" (`KismetMathLibrary.MakeTransform` spawn_location) "Undefined" "OverrideRootScale" null null))
  (set `self.newroad` _returnvalue))

(fn `spawn_grass_at _spawn_point`
  (`self.Spawn_Grass` (`SceneComponent.K2_GetComponentLocation` (`/Game/blueprints/BP_Grass.spawn_point` (`self.newgrass`)))))

(fn `Spawn_initial_grass`
  (for _ (range 5)
    (`/Engine/EditorBlueprintResources/StandardMacros.IsValid` (`self.newgrass`)
      (:`Is Valid`
        (`self.spawn_grass_at _spawn_point`))
      (:`Is Not Valid`
        (`self.Spawn_Grass` (0.0 0.0 0.0))))))

(fn `Spawn_Road`
  (params (spawn_location :type "Vector Structure"))
  (bind _returnvalue (`|SpawnActorFromClass` "/Game/blueprints/BP_Road.BP_Road_C" (`KismetMathLibrary.MakeTransform` spawn_location) "Undefined" "OverrideRootScale" null null))
  (bind _output_get (set `self.newroad` _returnvalue))
  (set `/Game/blueprints/BP_Road.Grass_Spawner` null _output_get))

(fn `spawn_road_at _spawn_point_0`
  (`self.Spawn_Road` (`SceneComponent.K2_GetComponentLocation` (`/Game/blueprints/BP_Road.spawn_point` (`self.newroad`)))))

(fn `UserConstructionScript`)