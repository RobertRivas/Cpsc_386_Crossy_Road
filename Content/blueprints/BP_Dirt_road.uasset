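; BP_Dirt_road is a road segment in the Crossy_Road game that spawns cars and triggers creation of the next segment.
; A latent Delay on Tick gives a randomly timed loop calling SpawnCar, which has even odds of spawning BP_Car at the right-side spawn point.
; Cars entering Car_respawn_zone are destroyed.
; When BP_Chicken enters Trigger_Zone, the game mode spawns another dirt road and this one destroys itself after a delay.
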(event `self.ReceiveBeginPlay`
  (`self.spawn_car`))

(event `self.ReceiveActorBeginOverlap`
  (params (OtherActor :type "Actor Object Reference")))

(event `self.ReceiveTick`
  (params (DeltaSeconds :type "Float (single-precision)"))
  (`KismetSystemLibrary.Delay` (`KismetMathLibrary.RandomFloatInRange` 0.5 1.0))
  (`self.spawn_car`))

(event `self.Trigger_Zone.OnComponentBeginOverlap`
  (params (OverlappedComponent :type "PrimitiveComponent Object Reference") (OtherActor :type "Actor Object Reference") (OtherComp :type "PrimitiveComponent Object Reference") (OtherBodyIndex :type Integer) (bFromSweep :type Boolean) (SweepResult :type "HitResult Structure (by ref)"))
  (cast `/Game/blueprints/BP_Chicken` OtherActor)
  (bind _ascrossy_road (cast `/Game/Crossy_Road` (`GameplayStatics.GetGameMode`)))
  (`/Game/Crossy_Road.Spawn_dirt_road` _ascrossy_road)
  (`KismetSystemLibrary.Delay` 5.0)
  (`self.K2_DestroyActor`))

(event `self.car_respawn_zone.OnComponentBeginOverlap`
  (params (OverlappedComponent :type "PrimitiveComponent Object Reference") (OtherActor :type "Actor Object Reference") (OtherComp :type "PrimitiveComponent Object Reference") (OtherBodyIndex :type Integer) (bFromSweep :type Boolean) (SweepResult :type "HitResult Structure (by ref)"))
  (bind _asbp_car (cast `/Game/blueprints/BP_Car` OtherActor))
  (`self.K2_DestroyActor` _asbp_car))

(fn `spawn_car`
  (switch `int` (`KismetMathLibrary.RandomIntegerInRange` 0 1)
    (:`1`
      (`|SpawnActorFromClass` "/Game/blueprints/BP_Car.BP_Car_C" (`SceneComponent.K2_GetComponentToWorld` (`self.right_side_spawn_point`)) "Undefined" "OverrideRootScale" null null))))

(fn `UserConstructionScript`)