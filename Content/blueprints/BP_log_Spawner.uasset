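; BP_log_Spawner is a spawner actor that builds a chain of BP_log actors end to end.
; SpawnLog stores the newest log and gives it a back-reference to the spawner, so each following log spawns at the previous one's LogSpawnPoint.
; SpawnInitialCar seeds four logs starting at the world origin, but nothing in this Blueprint calls it, as BeginPlay is empty.
; Disconnected leftover nodes hint at randomised road or log selection.
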(event `self.ReceiveBeginPlay`)

(event `self.ReceiveTick`
  (params (DeltaSeconds :type "Float (single-precision)")))

(fn `Spawn_initial_car`
  (for _ (range 4)
    (`/Engine/EditorBlueprintResources/StandardMacros.IsValid` (`self.newlog`)
      (:`Is Valid`
        (`self.spawn_log_at _spawn_point`))
      (:`Is Not Valid`
        (`self.Spawn_log` (0.0 0.0 0.0))))))

(fn `Spawn_log`
  (params (spawn_location :type "Vector Structure"))
  (bind _returnvalue (`|SpawnActorFromClass` "/Game/blueprints/BP_log.BP_log_C" (`KismetMathLibrary.MakeTransform` spawn_location) "Undefined" "OverrideRootScale" null null))
  (bind _output_get (set `self.newlog` _returnvalue))
  (set `/Game/blueprints/BP_log.log_spawner` self _output_get))

(fn `spawn_log_at _spawn_point`
  (`self.Spawn_log` (`SceneComponent.K2_GetComponentLocation` (`/Game/blueprints/BP_log.log spawn point` (`self.newlog`)))))

(fn `UserConstructionScript`)