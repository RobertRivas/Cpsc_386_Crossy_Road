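; Spawner actor that creates an initial chain of BP_Car actors when play begins.
; A short loop places the first car at the world origin, then each following one at the CarSpawnPoint component of the most recently spawned car.
; Each new car is stored as Newcar and given a reference back to this spawner.
; Disconnected leftover nodes for random checks and road spawning never run.
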(event `self.ReceiveBeginPlay`
  (`self.Spawn_initial_car`))

(event `self.ReceiveTick`
  (params (DeltaSeconds :type "Float (single-precision)")))

(fn `Spawn_Car`
  (params (spawn_location :type "Vector Structure"))
  (bind _returnvalue (`|SpawnActorFromClass` "/Game/blueprints/BP_Car.BP_Car_C" (`KismetMathLibrary.MakeTransform` spawn_location) "Undefined" "OverrideRootScale" null null))
  (bind _output_get (set `self.newcar` _returnvalue))
  (set `/Game/blueprints/BP_Car.car_spawner` self _output_get))

(fn `spawn_car_at _spawn_point`
  (`self.Spawn_Car` (`SceneComponent.K2_GetComponentLocation` (`/Game/blueprints/BP_Car.car spawn point` (`self.newcar`)))))

(fn `Spawn_initial_car`
  (for _ (range 4)
    (`/Engine/EditorBlueprintResources/StandardMacros.IsValid` (`self.newcar`)
      (:`Is Valid`
        (`self.spawn_car_at _spawn_point`))
      (:`Is Not Valid`
        (`self.Spawn_Car` (0.0 0.0 0.0))))))

(fn `UserConstructionScript`)