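; BP_train_Spawner builds the initial chain of BP_Train actors when play begins.
; A short loop spawns the first train at the world origin if none is valid, then places each next one at the previous train's TrainSpawnPoint.
; Each spawn becomes the stored Newtrain and receives a reference back to the spawner.
; A train whistle sound node is present but never runs.
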(event `self.ReceiveBeginPlay`
  (`self.Spawn_initial_train`))

(event `self.ReceiveTick`
  (params (DeltaSeconds :type "Float (single-precision)")))

(fn `Spawn_initial_train`
  (for _ (range 4)
    (`/Engine/EditorBlueprintResources/StandardMacros.IsValid` (`self.newtrain`)
      (:`Is Valid`
        (`self.spawn_train_at _spawn_point`))
      (:`Is Not Valid`
        (`self.Spawn_train` (0.0 0.0 0.0))))))

(fn `Spawn_train`
  (params (spawn_location :type "Vector Structure"))
  (bind _returnvalue (`|SpawnActorFromClass` "/Game/blueprints/BP_Train.BP_Train_C" (`KismetMathLibrary.MakeTransform` spawn_location) "Undefined" "OverrideRootScale" null null))
  (bind _output_get (set `self.newtrain` _returnvalue))
  (set `/Game/blueprints/BP_Train.train_spawner` self _output_get))

(fn `spawn_train_at _spawn_point`
  (`self.Spawn_train` (`SceneComponent.K2_GetComponentLocation` (`/Game/blueprints/BP_Train.Train spawn point` (`self.newtrain`)))))

(fn `UserConstructionScript`)