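; Bus spawner Blueprint that builds a short chain of BP_bus actors.
; SpawnInitialBus loops, placing a bus at the origin if none is valid, otherwise at the last bus's BusSpawnPoint.
; SpawnBus stores each new actor in Newbus, so the next spawn attaches positionally to it.
; Nothing calls SpawnInitialBus from a live event, and leftover random and road-spawning nodes are disconnected.
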(event `self.ReceiveBeginPlay`)

(event `self.ReceiveTick`
  (params (DeltaSeconds :type "Float (single-precision)")))

(fn `Spawn_bus`
  (params (spawn_location :type "Vector Structure"))
  (bind _returnvalue (`|SpawnActorFromClass` "/Game/blueprints/BP_bus.BP_bus_C" (`KismetMathLibrary.MakeTransform` spawn_location) "Undefined" "OverrideRootScale" null null))
  (set `self.newbus` _returnvalue))

(fn `spawn_bus_at _spawn_point`
  (`self.Spawn_bus` (`SceneComponent.K2_GetComponentLocation` (`/Game/blueprints/BP_bus.Bus spawn point` (`self.newbus`)))))

(fn `Spawn_initial_bus`
  (for _ (range 4)
    (`/Engine/EditorBlueprintResources/StandardMacros.IsValid` (`self.newbus`)
      (:`Is Valid`
        (`self.spawn_bus_at _spawn_point`))
      (:`Is Not Valid`
        (`self.Spawn_bus` (0.0 0.0 0.0))))))

(fn `UserConstructionScript`)